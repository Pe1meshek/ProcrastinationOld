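; BP_Pirat is the 2D pirate actor that spawns and kicks Pinus projectiles, and triggers the lose screen on touching a BP_DeadLine.
; Input spawns the selected Pinus variant, starts a charge flipbook whose playback frame sets kick power, or activates the current Pinus.
; After a delay timed to the attack flipbook, Pinus actors in the attack box receive an X/Z impulse based on that power and cursor direction.
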(event `self.ReceiveTick`
  (params (DeltaSeconds :type "Float (single-precision)")))

(event `self.ReceiveBeginPlay`
  (`PaperFlipbookComponent.SetLooping` (`self.PaperFlipbook`) false)
  (`PaperFlipbookComponent.SetLooping` (`self.PF_Charge`) false))

(event `EnhancedInput|/Game/input/IA_PinusFocusSkip`
  (params (ActionValue :type Boolean) (ElapsedSeconds :type "Float (double-precision)") (TriggeredSeconds :type "Float (double-precision)") (InputAction :type "InputAction Object Reference" :default "/Game/input/IA_PinusFocusSkip.IA_PinusFocusSkip"))
  (bind _output (`|ConvertAsset` (`self.ref_Pinus`)))
  (bind _bp_arrow (`/Game/bp/Pinus/BP_Pinus.BP_Arrow` _output))
  (:`Triggered`
    (`/Engine/EditorBlueprintResources/StandardMacros.IsValid` _output
      (:`Is Valid`
        (`/Engine/EditorBlueprintResources/StandardMacros.IsValid` _bp_arrow
          (:`Is Valid`
            (`self.K2_DestroyActor` _bp_arrow))
          (:`Is Not Valid`
            _))
        (set `self.isPinusCreated` false)))))

(event `self.PaperFlipbook.OnFinishedPlaying`
  (bind _paperflipbook (`self.PaperFlipbook`))
  (`PaperFlipbookComponent.SetLooping` _paperflipbook true)
  (`PaperFlipbookComponent.SetFlipbook` _paperflipbook "/Game/bp/Pinala/idle.idle")
  (`PaperFlipbookComponent.Play` _paperflipbook))

(event `EnhancedInput|/Game/input/IA_Piu`
  (params (ActionValue :type Boolean) (ElapsedSeconds :type "Float (double-precision)") (TriggeredSeconds :type "Float (double-precision)") (InputAction :type "InputAction Object Reference" :default "/Game/input/IA_Piu.IA_Piu"))
  (bind _paperflipbook (`self.PaperFlipbook`))
  (:`Triggered`
    (bind _result (`/Engine/EditorBlueprintResources/StandardMacros.IncrementInt` (`PaperFlipbookComponent.GetPlaybackPositionInFrames` (`self.PF_Charge`)))
      (:`  `
        (set `self.kickPower` _result)
        (if (`self.canKick`)
          (set `self.canKick` false)
          (`PaperFlipbookComponent.SetLooping` _paperflipbook false)
          (`PaperFlipbookComponent.SetFlipbook` _paperflipbook "/Game/bp/Pinala/attack.attack")
          (`PaperFlipbookComponent.PlayFromStart` _paperflipbook)
          (`SceneComponent.SetVisibility` (`self.PF_Charge`) false false)
          (`KismetSystemLibrary.Delay` (- (`PaperFlipbookComponent.GetFlipbookLength` _paperflipbook) 0.4))
          (`self.kickPinus`))))))

(event `EnhancedInput|/Game/input/IA_Charge`
  (params (ActionValue :type Boolean) (ElapsedSeconds :type "Float (double-precision)") (TriggeredSeconds :type "Float (double-precision)") (InputAction :type "InputAction Object Reference" :default "/Game/input/IA_Charge.IA_Charge"))
  (bind _pf_charge (`self.PF_Charge`))
  (:`Triggered`
    (if (`self.canKick`)
      (`SceneComponent.SetVisibility` _pf_charge true false)
      (`PaperFlipbookComponent.PlayFromStart` _pf_charge))))

(event `self.PF_Charge.OnFinishedPlaying`
  (bind _pf_charge (`self.PF_Charge`))
  (bind _paperflipbook (`self.PaperFlipbook`))
  (bind _result (`/Engine/EditorBlueprintResources/StandardMacros.IncrementInt` (`PaperFlipbookComponent.GetPlaybackPositionInFrames` _pf_charge))
    (:`  `
      (set `self.kickPower` _result)
      (`SceneComponent.SetVisibility` _pf_charge false false)
      (if (`self.canKick`)
        (set `self.canKick` false)
        (`PaperFlipbookComponent.SetLooping` _paperflipbook false)
        (`PaperFlipbookComponent.SetFlipbook` _paperflipbook "/Game/bp/Pinala/attack.attack")
        (`PaperFlipbookComponent.PlayFromStart` _paperflipbook)
        (`KismetSystemLibrary.Delay` (- (`PaperFlipbookComponent.GetFlipbookLength` _paperflipbook) 0.4))
        (`self.kickPinus`)))))

(event `Key|C`
  (params (Key :type "Key Structure")))

(event `EnhancedInput|/Game/input/IA_CreatePinus`
  (params (ActionValue :type Boolean) (ElapsedSeconds :type "Float (double-precision)") (TriggeredSeconds :type "Float (double-precision)") (InputAction :type "InputAction Object Reference" :default "/Game/input/IA_CreatePinus.IA_CreatePinus"))
  (:`Triggered`
    (`self.createPinus`)
    (set `self.canKick` true)))

(event `EnhancedInput|/Game/input/IA_PinusActivate`
  (params (ActionValue :type Boolean) (ElapsedSeconds :type "Float (double-precision)") (TriggeredSeconds :type "Float (double-precision)") (InputAction :type "InputAction Object Reference" :default "/Game/input/IA_PinusActivate.IA_PinusActivate"))
  (bind _output (`|ConvertAsset` (`self.ref_Pinus`)))
  (:`Triggered`
    (`/Engine/EditorBlueprintResources/StandardMacros.IsValid` _output
      (:`Is Valid`
        (`/Game/bp/Pinus/BP_Pinus.pinusActivate` _output)))))

(event `self.ReceiveActorBeginOverlap`
  (params (OtherActor :type "Actor Object Reference"))
  (cast `/Game/bp/DeadLine/BP_DeadLine` OtherActor)
  (bind _aspc_ (cast `/Game/PC_` (`GameplayStatics.GetPlayerController` 0)))
  (`/Game/PC_.createLoseGameWB` _aspc_)
  (`GameplayStatics.SetGamePaused` true))

(fn `createPinus`
  (if (not (not (`self.isPinusCreated`)))
    (`/Game/bp/Pinus/BP_Pinus.unReferencePirat` (`|ConvertAsset` (`self.ref_Pinus`))))
  (bind _pinusclass (`self.numToPinusClass` (`self.numSelectPinus`)))
  (bind _returnvalue (`|SpawnActorFromClass` _pinusclass (`KismetMathLibrary.MakeTransform` (`SceneComponent.K2_GetComponentLocation` (`self.pinusSpawnPoint`)) (struct) (0.1 0.1 0.1)) "Undefined" "MultiplyWithRoot" null null))
  (set `self.ref_Pinus` (`|ConvertAsset` _returnvalue))
  (set `self.isPinusCreated` true)
  (bind _returnvalue_2 (`GameplayStatics.GetActorOfClass` "/Game/bp/Camera/BP_Camera.BP_Camera_C"))
  (`/Game/bp/Camera/BP_Camera.savePinus` _returnvalue_2))

(fn `kickPinus`
  (bind _returnvalue (`GameplayStatics.GetPlayerController` 0))
  (bind _returnvalue_2 (`self.GetDistanceTo` _returnvalue))
  (bind _returnvalue_3 (* (`self.kickPower`) (`self.kofKickPower`)))
  (bind (_returnvalue_x _returnvalue_y _returnvalue_z) (`KismetMathLibrary.BreakVector` (- (`.Location` (`GameplayStatics.BreakHitResult` (`PlayerController.GetHitResultUnderCursorByChannel` _returnvalue "TraceTypeQuery3" true))) (`self.K2_GetActorLocation`))))
  (for _array_element (`PrimitiveComponent.GetOverlappingActors` (`self.boxAttack`) "/Game/bp/Pinus/BP_Pinus.BP_Pinus_C")
    (bind _asbp_pinus (cast `/Game/bp/Pinus/BP_Pinus` _array_element))
    (bind _bp_arrow (`/Game/bp/Pinus/BP_Pinus.BP_Arrow` _asbp_pinus))
    (`/Engine/EditorBlueprintResources/StandardMacros.IsValid` _bp_arrow
      (:`Is Valid`
        (`self.K2_DestroyActor` _bp_arrow))
      (:`Is Not Valid`
        _))
    (set `/Game/bp/Pinus/BP_Pinus.isKicked` true _asbp_pinus)
    (`/Game/bp/Pinus/BP_Pinus.Event Kick` _asbp_pinus)
    (`PrimitiveComponent.AddImpulseAtLocation` (`/Game/bp/Pinus/BP_Pinus.Capsule` _asbp_pinus) (`KismetMathLibrary.MakeVector` (* _returnvalue_3 (/ _returnvalue_x _returnvalue_2)) 0.0 (* _returnvalue_3 (/ _returnvalue_z _returnvalue_2))) (0.0 0.0 0.0) "None")))

(fn `numToPinusClass`
  (params (num :type Integer))
  (returns (PinusClass :type "/Game/bp/Pinus/BP_Pinus Class Reference"))
  (switch `int` num
    (:`Default`
      _)
    (:`0`
      _)
    (:`1`
      (return "/Game/bp/Pinus/BP_HellPinus.BP_HellPinus_C"))
    (:`2`
      (return "/Game/bp/Pinus/BP_MagnetPinus.BP_MagnetPinus_C")))
  (return "/Game/bp/Pinus/BP_Pinus.BP_Pinus_C"))

(fn `UserConstructionScript`)