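; Shared camera actor that keeps the Pirat player character, Delo, Varp and, once created, Pinus framed together in the XZ plane.
; BeginPlay caches references to these actors, taking Pinus from the Pirat.
; While AutoMode is on, Tick runs AllFocus, which centers the actor on their bounding extents.
; It sets the camera's relative Y from the larger weighted X or Z spread, zooming as they separate.
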(event `self.ReceiveBeginPlay`
  (bind _returnvalue (`GameplayStatics.GetActorOfClass` "/Game/bp/Delo/BP_Delo.BP_Delo_C"))
  (set `self.refDelo` (`|ConvertAsset` _returnvalue))
  (bind _returnvalue_2 (`GameplayStatics.GetActorOfClass` "/Game/bp/Varp/BP_Varp.BP_Varp_C"))
  (set `self.refVarp` (`|ConvertAsset` _returnvalue_2))
  (bind _asbp_pirat (cast `/Game/bp/Pinala/BP_Pirat` (`GameplayStatics.GetPlayerCharacter` 0)))
  (set `self.refPirat` (`|ConvertAsset` _asbp_pirat))
  (`self.savePinus`))

(event `self.ReceiveActorBeginOverlap`
  (params (OtherActor :type "Actor Object Reference")))

(event `self.ReceiveTick`
  (params (DeltaSeconds :type "Float (single-precision)"))
  (if (`self.autoMode`)
    (`self.allFocus`)))

(fn `allFocus`
  (locals (minX :type "Float (double-precision)") (maxX :type "Float (double-precision)") (minZ :type "Float (double-precision)") (maxZ :type "Float (double-precision)"))
  (bind _output (`|ConvertAsset` (`self.refPirat`)))
  (bind _output_2 (`|ConvertAsset` (`self.refPinus`)))
  (bind (_returnvalue_x _returnvalue_y _returnvalue_z) (`KismetMathLibrary.BreakVector` (`self.K2_GetActorLocation` _output_2)))
  (bind (_returnvalue_x_2 _returnvalue_y_2 _returnvalue_z_2) (`KismetMathLibrary.BreakVector` (`self.K2_GetActorLocation` (`|ConvertAsset` (`self.refDelo`)))))
  (bind (_returnvalue_x_3 _returnvalue_y_3 _returnvalue_z_3) (`KismetMathLibrary.BreakVector` (`self.K2_GetActorLocation` (`|ConvertAsset` (`self.refVarp`)))))
  (bind (_returnvalue_x_4 _returnvalue_y_4 _returnvalue_z_4) (`KismetMathLibrary.BreakVector` (`self.K2_GetActorLocation` _output)))
  (bind _returnvalue (`KismetMathLibrary.FMin` _returnvalue_z_4 _returnvalue_z _returnvalue_z_2 _returnvalue_z_3))
  (bind _returnvalue_2 (`KismetMathLibrary.FMin` _returnvalue_z_4 _returnvalue_z_2 _returnvalue_z_3))
  (bind _returnvalue_3 (`KismetMathLibrary.FMin` _returnvalue_x_4 _returnvalue_x _returnvalue_x_2 _returnvalue_x_3))
  (bind _returnvalue_4 (`KismetMathLibrary.FMin` _returnvalue_x_4 _returnvalue_x_2 _returnvalue_x_3))
  (bind _returnvalue_5 (`KismetMathLibrary.Abs` (- (`KismetMathLibrary.FMax` _returnvalue_z_4 _returnvalue_z_2 _returnvalue_z_3) _returnvalue_2)))
  (bind _returnvalue_6 (`KismetMathLibrary.Abs` (- (`KismetMathLibrary.FMax` _returnvalue_z_4 _returnvalue_z _returnvalue_z_2 _returnvalue_z_3) _returnvalue)))
  (bind _returnvalue_7 (`KismetMathLibrary.Abs` (- (`KismetMathLibrary.FMax` _returnvalue_x_4 _returnvalue_x _returnvalue_x_2 _returnvalue_x_3) _returnvalue_3)))
  (bind _returnvalue_8 (`KismetMathLibrary.Abs` (- (`KismetMathLibrary.FMax` _returnvalue_x_4 _returnvalue_x_2 _returnvalue_x_3) _returnvalue_4)))
  (`/Engine/EditorBlueprintResources/StandardMacros.IsValid` _output_2
    (:`Is Valid`
      (if (`/Game/bp/Pinala/BP_Pirat.isPinusCreated` _output)
        (`self.K2_SetActorLocation` (`KismetMathLibrary.MakeVector` (+ _returnvalue_3 (/ _returnvalue_7 2.0)) 0.0 (+ _returnvalue (/ _returnvalue_6 2.0))))
        (`SceneComponent.K2_SetRelativeLocation` (`self.Camera`) (`KismetMathLibrary.MakeVector` 0.0 (`KismetMathLibrary.FMax` (* _returnvalue_7 0.625) (* _returnvalue_6 1.0))) false false)
        (else
          (`self.K2_SetActorLocation` (`KismetMathLibrary.MakeVector` (+ _returnvalue_4 (/ _returnvalue_8 2.0)) 0.0 (+ _returnvalue_2 (/ _returnvalue_5 2.0))) :!label _label)
          (`SceneComponent.K2_SetRelativeLocation` (`self.Camera`) (`KismetMathLibrary.MakeVector` 0.0 (`KismetMathLibrary.FMax` (* _returnvalue_8 0.625) (* _returnvalue_5 1.0))) false false))))
    (:`Is Not Valid`
      (goto _label))))

(fn `savePinus`
  (set `self.refPinus` (`/Game/bp/Pinala/BP_Pirat.ref_Pinus` (`|ConvertAsset` (`self.refPirat`)))))

(fn `UserConstructionScript`)