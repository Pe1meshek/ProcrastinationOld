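; Spike variant of a Pinus actor that bursts into eight new BP_Pinus actors when activated.
; It overrides PinusActivate and, if the parent call succeeds, spawns one at each of eight directional components.
; Each spawn has its BPArrow actor destroyed and its capsule pushed outward in the X-Z plane, using the cosine and sine of that component's relative pitch.
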(fn `pinusActivate`
  (returns (aceivate :type Boolean))
  (bind _aceivate (`parent.pinusActivate`))
  (if _aceivate
    (for _array_element (`|MakeArray` (`self.LeftUp`) (`self.LeftDown`) (`self.RightUp`) (`self.RightDown`) (`self.Right`) (`self.Left`) (`self.Down`) (`self.Up`))
      (bind _returnvalue (`|SpawnActorFromClass` "/Game/bp/Pinus/BP_Pinus.BP_Pinus_C" (`SceneComponent.K2_GetComponentToWorld` _array_element) "AlwaysSpawn" "MultiplyWithRoot" null null))
      (`self.K2_DestroyActor` (`/Game/bp/Pinus/BP_Pinus.BP_Arrow` _returnvalue))
      (bind (_relativerotation_roll _relativerotation_pitch) (`KismetMathLibrary.BreakRotator` (`SceneComponent.RelativeRotation` _array_element)))
      (`PrimitiveComponent.AddImpulse` (`/Game/bp/Pinus/BP_Pinus.Capsule` _returnvalue) (`KismetMathLibrary.MakeVector` (* (`KismetMathLibrary.DegCos` _relativerotation_pitch) 200.0) 0.0 (* (`KismetMathLibrary.DegSin` _relativerotation_pitch) 200.0)) "None" false))))

(fn `UserConstructionScript`
  (`parent.UserConstructionScript`))