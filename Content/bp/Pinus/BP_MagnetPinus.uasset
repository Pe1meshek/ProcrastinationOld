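; BP_MagnetPinus is a Pinus variant that, once activated, fires a magnetic pulse pulling BP_Delo actors toward itself.
; PinusActivate runs the parent check, then shows the MagnetPole sphere, enables its collision at the starting radius and starts a fast looping timer.
; MagnetPoleAction shrinks the sphere each step, applying distance-scaled impulses to overlapping Delo capsules until it collapses, then clears the timer and hides the sphere.
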(event `self.ReceiveBeginPlay`
  (bind _magnetpole (`self.magnetPole`))
  (`parent.ReceiveBeginPlay`)
  (`SceneComponent.SetVisibility` _magnetpole false false)
  (`PrimitiveComponent.SetCollisionEnabled` _magnetpole "NoCollision"))

(event `self.magnetPole.OnComponentBeginOverlap`
  (params (OverlappedComponent :type "PrimitiveComponent Object Reference") (OtherActor :type "Actor Object Reference") (OtherComp :type "PrimitiveComponent Object Reference") (OtherBodyIndex :type Integer) (bFromSweep :type Boolean) (SweepResult :type "HitResult Structure (by ref)")))

(event `self.magnetPole.OnComponentEndOverlap`
  (params (OverlappedComponent :type "PrimitiveComponent Object Reference") (OtherActor :type "Actor Object Reference") (OtherComp :type "PrimitiveComponent Object Reference") (OtherBodyIndex :type Integer)))

(fn `magnetPoleAction`
  (bind _magnetpole (`self.magnetPole`))
  (bind _magnetpole_2 (`self.magnetPole`))
  (bind _returnvalue (- (`SphereComponent.SphereRadius` _magnetpole_2) 50.0))
  (`SphereComponent.SetSphereRadius` _magnetpole_2 _returnvalue true)
  (if (< _returnvalue 2.0)
    (`KismetSystemLibrary.K2_ClearAndInvalidateTimerHandle` (`self.magnetPoleActionHandler`))
    (`SceneComponent.SetVisibility` _magnetpole false false)
    (`PrimitiveComponent.SetCollisionEnabled` _magnetpole "NoCollision")
    (else
      (for _array_element (`PrimitiveComponent.GetOverlappingActors` _magnetpole_2 "/Game/bp/Delo/BP_Delo.BP_Delo_C")
        (bind _asbp_delo (cast `/Game/bp/Delo/BP_Delo` _array_element))
        (`PrimitiveComponent.AddImpulse` (`/Game/bp/Delo/BP_Delo.Capsule` _asbp_delo) (* (- (`self.K2_GetActorLocation`) (`self.K2_GetActorLocation` _asbp_delo)) 20) "None" false)))))

(fn `pinusActivate`
  (returns (aceivate :type Boolean))
  (bind _magnetpole (`self.magnetPole`))
  (bind _aceivate (`parent.pinusActivate`))
  (if _aceivate
    (`SceneComponent.SetVisibility` _magnetpole true false)
    (`PrimitiveComponent.SetCollisionEnabled` _magnetpole "QueryAndPhysics")
    (`SphereComponent.SetSphereRadius` _magnetpole (`self.START_POLE_RADIUS`) true)
    (bind _returnvalue (`KismetSystemLibrary.K2_SetTimerDelegate` (`|CreateDelegate` :!event `magnetPoleAction`) 0.005 true true))
    (set `self.magnetPoleActionHandler` _returnvalue)))

(fn `UserConstructionScript`
  (`parent.UserConstructionScript`))