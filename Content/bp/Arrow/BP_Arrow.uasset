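; BP_Arrow is an arrow actor that tilts to follow the mouse cursor around the viewport center.
; Each Tick sets its pitch to the arcsine of the cursor's vertical offset over its distance from center.
; This confines pitch to ±90 degrees, so cursor positions mirrored left and right give the same angle.
; Disconnected debug prints and an alternative MakeRotFromZX rotation remain unused in the graph.
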(event `self.ReceiveTick`
  (params (DeltaSeconds :type "Float (single-precision)"))
  (bind (_returnvalue_x _returnvalue_y) (`KismetMathLibrary.BreakVector2D` (`WidgetLayoutLibrary.GetViewportSize`)))
  (bind _returnvalue (`WidgetLayoutLibrary.GetMousePositionOnViewport`))
  (bind _returnvalue_2 (- (/ _returnvalue_y 2.0) (`.Y` (`KismetMathLibrary.BreakVector2D` _returnvalue))))
  (`self.K2_SetActorRotation` (`KismetMathLibrary.MakeRotator` 0.0 (`KismetMathLibrary.DegAsin` (/ _returnvalue_2 (`KismetMathLibrary.Sqrt` (+ (`KismetMathLibrary.MultiplyMultiply_FloatFloat` (- (`KismetMathLibrary.BreakVector2D` _returnvalue) (/ _returnvalue_x 2.0)) 2.0) (`KismetMathLibrary.MultiplyMultiply_FloatFloat` _returnvalue_2 2.0))))))))

(fn `UserConstructionScript`)