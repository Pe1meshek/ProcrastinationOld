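; Player controller that sets up input, cursor and UI, and drives the level's BP_Camera as the view target.
; BeginPlay creates hidden pause and controls widgets; IA_Pause toggles the pause menu and game pause.
; Outside AutoMode, inputs pan the camera along X and Z, scaled by its Y zoom offset, which scroll changes unclamped.
; A flip-flop input switches AutoMode, and two functions spawn lose and level-complete screens.
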(event `self.ReceiveBeginPlay`
  (bind _returnvalue (`GameplayStatics.GetPlayerController` 0))
  (`/Engine/EditorBlueprintResources/StandardMacros.IsValid` _returnvalue
    (:`Is Valid`
      (`EnhancedInputSubsystemInterface.AddMappingContext` (pcsubsystem `EnhancedInputLocalPlayerSubsystem` _returnvalue) "/Game/input/IMC_Based.IMC_Based" 0 (struct))
      (set `PlayerController.bShowMouseCursor` true _returnvalue)
      (bind _returnvalue_2 (`|CreateWidget` "/Game/UI/WB_PauseMenu.WB_PauseMenu_C"))
      (bind _output_get (set `self.WPauseMenu` _returnvalue_2))
      (`UserWidget.AddToViewport` _output_get 0)
      (set `Widget.Visibility` "Hidden" _returnvalue_2)
      (bind _returnvalue_3 (`|CreateWidget` "/Game/UI/WB_Controls.WB_Controls_C"))
      (set `/Game/UI/WB_PauseMenu.ref_WB_Control` (`|ConvertAsset` _returnvalue_3) (`self.WPauseMenu`))
      (`UserWidget.AddToViewport` _returnvalue_3 0)
      (set `Widget.Visibility` "Hidden" _returnvalue_3)
      (bind _returnvalue_4 (`GameplayStatics.GetActorOfClass` "/Game/bp/Camera/BP_Camera.BP_Camera_C"))
      (`self.SetViewTargetWithBlend` _returnvalue_4 0.3)
      (bind _asbp_camera (cast `/Game/bp/Camera/BP_Camera` _returnvalue_4))
      (set `self.refCamera` (`|ConvertAsset` _asbp_camera)))))

(event `EnhancedInput|/Game/input/IA_Pause`
  (params (ActionValue :type Boolean) (ElapsedSeconds :type "Float (double-precision)") (TriggeredSeconds :type "Float (double-precision)") (InputAction :type "InputAction Object Reference" :default "/Game/input/IA_Pause.IA_Pause"))
  (bind _wpausemenu (`self.WPauseMenu`))
  (bind _returnvalue (`Widget.IsVisible` _wpausemenu))
  (:`Triggered`
    (`GameplayStatics.SetGamePaused` (not _returnvalue))
    (if _returnvalue
      (set `Widget.Visibility` "Hidden" _wpausemenu)
      (else
        (set `Widget.Visibility` "Visible" _wpausemenu)))))

(event `Key|Escape`
  (params (Key :type "Key Structure")))

(event `Key|Tab`
  (params (Key :type "Key Structure")))

(event `EnhancedInput|/Game/input/IA_HorizontMove`
  (params (ActionValue :type "Float (double-precision)") (ElapsedSeconds :type "Float (double-precision)") (TriggeredSeconds :type "Float (double-precision)") (InputAction :type "InputAction Object Reference" :default "/Game/input/IA_HorizontMove.IA_HorizontMove"))
  (bind _output (`|ConvertAsset` (`self.refCamera`)))
  (bind (_returnvalue_x _returnvalue_y _returnvalue_z) (`KismetMathLibrary.BreakVector` (`self.K2_GetActorLocation` _output)))
  (bind (_relativelocation_x _relativelocation_y) (`KismetMathLibrary.BreakVector` (`SceneComponent.RelativeLocation` (`/Game/bp/Camera/BP_Camera.Camera` _output))))
  (:`Triggered`
    (if (not (`/Game/bp/Camera/BP_Camera.autoMode` _output))
      (`self.K2_SetActorLocation` _output (`KismetMathLibrary.MakeVector` (+ _returnvalue_x (* ActionValue (/ _relativelocation_y 50.0))) _returnvalue_y _returnvalue_z) false false))))

(event `EnhancedInput|/Game/input/IA_Scroll`
  (params (ActionValue :type "Float (double-precision)") (ElapsedSeconds :type "Float (double-precision)") (TriggeredSeconds :type "Float (double-precision)") (InputAction :type "InputAction Object Reference" :default "/Game/input/IA_Scroll.IA_Scroll"))
  (bind _camera (`/Game/bp/Camera/BP_Camera.Camera` (`|ConvertAsset` (`self.refCamera`))))
  (bind (_relativelocation_x _relativelocation_y _relativelocation_z) (`KismetMathLibrary.BreakVector` (`SceneComponent.RelativeLocation` _camera)))
  (:`Triggered`
    (if (not (`/Game/bp/Camera/BP_Camera.autoMode` (`|ConvertAsset` (`self.refCamera`))))
      (`SceneComponent.K2_SetRelativeLocation` _camera (`KismetMathLibrary.MakeVector` _relativelocation_x (+ (* ActionValue -50.0) _relativelocation_y) _relativelocation_z) false false))))

(event `EnhancedInput|/Game/input/IA_VerticalMove`
  (params (ActionValue :type "Float (double-precision)") (ElapsedSeconds :type "Float (double-precision)") (TriggeredSeconds :type "Float (double-precision)") (InputAction :type "InputAction Object Reference" :default "/Game/input/IA_VerticalMove.IA_VerticalMove"))
  (bind _output (`|ConvertAsset` (`self.refCamera`)))
  (bind (_returnvalue_x _returnvalue_y _returnvalue_z) (`KismetMathLibrary.BreakVector` (`self.K2_GetActorLocation` _output)))
  (bind (_relativelocation_x _relativelocation_y) (`KismetMathLibrary.BreakVector` (`SceneComponent.RelativeLocation` (`/Game/bp/Camera/BP_Camera.Camera` _output))))
  (:`Triggered`
    (if (not (`/Game/bp/Camera/BP_Camera.autoMode` _output))
      (`self.K2_SetActorLocation` _output (`KismetMathLibrary.MakeVector` _returnvalue_x _returnvalue_y (+ _returnvalue_z (* ActionValue (/ _relativelocation_y 50.0)))) false false))))

(event `EnhancedInput|/Game/input/IA_FlipCameraMode`
  (params (ActionValue :type Boolean) (ElapsedSeconds :type "Float (double-precision)") (TriggeredSeconds :type "Float (double-precision)") (InputAction :type "InputAction Object Reference" :default "/Game/input/IA_FlipCameraMode.IA_FlipCameraMode"))
  (:`Triggered`
    (bind _isa (`/Engine/EditorBlueprintResources/StandardMacros.FlipFlop`)
      (:`A`
        _)
      (:`B`
        _))
    (set `/Game/bp/Camera/BP_Camera.autoMode` (not _isa) (`|ConvertAsset` (`self.refCamera`)))))

(fn `createCompliteLevelWB`
  (bind _returnvalue (`|CreateWidget` "/Game/UI/WB_LevelComplite.WB_LevelComplite_C"))
  (`UserWidget.AddToViewport` _returnvalue 0))

(fn `createLoseGameWB`
  (bind _returnvalue (`|CreateWidget` "/Game/UI/WB_LoseGame.WB_LoseGame_C"))
  (`UserWidget.AddToViewport` _returnvalue 0))

(fn `UserConstructionScript`)